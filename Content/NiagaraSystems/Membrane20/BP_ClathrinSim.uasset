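; Simulation actor that builds a clathrin assembly from origin, Euler-angle and control-point data at BeginPlay.
; Spawns a randomly colored skeletal mesh per clathrin, converting source coordinates by flipping axes and scaling positions.
; Six physics handles per mesh grab the leg bones and target that clathrin's control points, so physics pulls the legs into shape.
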(event EventBeginPlay
  (bind _returnvalue (Class|ClathrinSim|GetClathrinOrigins))
  (bind _output_get (Variables|Default|SetClathrinOrigins _returnvalue))
  (bind _returnvalue_2 (Class|ClathrinSim|GetClathrinEulerAngles))
  (bind _output_get_2 (Variables|Default|SetEulerAngles _returnvalue_2))
  (bind _returnvalue_3 (Class|ClathrinSim|GetClathrinCtrlPoints))
  (Variables|Default|SetCtrlPoints _returnvalue_3)
  (bind (_array_element _array_index) (Utilities|Array|ForEachLoopwithBreak _output_get)
    (:LoopBody
      (bind _outpos (CallFunction|GetProperPosition _array_element))
      (bind _returnvalue_4 (AddComponent|AddSkeletalMeshComponent false (Math|Transform|MakeTransform _outpos (Class|KismetMathLibrary|QuatRotator (Class|KismetMathLibrary|QuatMakefromEuler (Math|Vector|MakeVector (Math|Trig|RadiansToDegrees (.X (Math|Vector|BreakVector (* (Utilities|Array|Get(acopy) _output_get_2 _array_index) "1.000000,-1.000000,-1.000000")))) (Math|Trig|RadiansToDegrees (.Y (Math|Vector|BreakVector (* (Utilities|Array|Get(acopy) _output_get_2 _array_index) "1.000000,-1.000000,-1.000000")))) (Math|Trig|RadiansToDegrees (.Z (Math|Vector|BreakVector (* (Utilities|Array|Get(acopy) _output_get_2 _array_index) "1.000000,-1.000000,-1.000000"))))))) (Math|Conversions|ToVector(Float) (Variables|Default|GetMeshUnitScale)))))
      (bind _returnvalue_5 (Rendering|Material|CreateDynamicMaterialInstance "/Game/NiagaraSystems/Membrane20/ClathrinMesh/v1/Mat_Clathrin.Mat_Clathrin" "None" "None" :!class /Script/Engine.KismetMaterialLibrary))
      (Rendering|Material|SetVectorParameterValue _returnvalue_5 "Color" (Utilities|Struct|MakeLinearColor (Math|Random|RandomFloat) (Math|Random|RandomFloat) (Math|Random|RandomFloat) 1.0) :!class /Script/Engine.MaterialInstanceDynamic)
      (Rendering|Material|SetMaterial _returnvalue_4 0 _returnvalue_5)
      (CallFunction|CreateClathrinPhysicsHandle _returnvalue_4 (Variables|Default|GetBN_Leg1_1) _array_index)
      (CallFunction|CreateClathrinPhysicsHandle _returnvalue_4 (Variables|Default|GetBN_Leg2_1) _array_index 2)
      (CallFunction|CreateClathrinPhysicsHandle _returnvalue_4 (Variables|Default|GetBN_Leg3_1) _array_index 1)
      (CallFunction|CreateClathrinPhysicsHandle _returnvalue_4 (Variables|Default|GetBN_Leg1_2) _array_index 4)
      (CallFunction|CreateClathrinPhysicsHandle _returnvalue_4 (Variables|Default|GetBN_Leg2_2) _array_index 3)
      (CallFunction|CreateClathrinPhysicsHandle _returnvalue_4 (Variables|Default|GetBN_Leg3_2) _array_index 5))))

(event Collision|EventActorBeginOverlap
  (params (OtherActor :type Actor%20Object%20Reference)))

(event EventTick
  (params (DeltaSeconds :type Float%20%28single-precision%29)))

(fn ConstructionScript)

(fn GetProperPosition
  (params (InPos :type Vector))
  (return (* (* InPos "1.000000,-1.000000,1.000000") (Variables|Default|GetPositionUnitScale))))

(fn CreateClathrinPhysicsHandle
  (params (SkeletalMeshComp :type Skeletal%20Mesh%20Component%20Object%20Reference) (BoneName :type Name) (ClathrinIndex :type Integer) (CtrlPointIndex :type Integer))
  (bind _returnvalue (AddComponent|AddPhysicsHandleComponent))
  (Class|PhysicsHandleComponent|GrabComponentatLocation _returnvalue SkeletalMeshComp BoneName (Transformation|GetSocketLocation SkeletalMeshComp BoneName))
  (bind _outpos (CallFunction|GetProperPosition (Utilities|Array|Get(acopy) (Variables|Default|GetCtrlPoints) (+ (* ClathrinIndex 6) CtrlPointIndex))))
  (Physics|Components|PhysicsHandle|SetTargetLocation _returnvalue _outpos))