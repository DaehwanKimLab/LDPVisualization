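; Manager actor for the Niagara molecule emitter that writes molecule event data into the RT_Events render target on BeginPlay.
; DrawToEventRenderTarget packs two hardcoded event structs into three colors each: molecule types, end location and end quaternion.
; It draws each color as an opaque 1x1 canvas quad along the top row, turning the texture into a data buffer.
; The struct conversion helper functions are unused stubs.
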(event EventBeginPlay
  (CallFunction|DrawtoEventRenderTarget))

(event Collision|EventActorBeginOverlap
  (params (OtherActor :type Actor%20Object%20Reference)))

(event EventTick
  (params (DeltaSeconds :type Float%20%28single-precision%29)))

(fn ConstructionScript)

(fn DrawtoEventRenderTarget
  (bind _vector4 (Math|Vector4|MakeVector4 0.0 0.0 0.0 0.0))
  (bind _vector4_2 (Math|Vector4|MakeVector4 0.0 0.0 0.0 0.0))
  (bind _s_eventstruct (Utilities|Struct|MakeS_EventStruct 1 2 "1.000000,20.000000,10.000000" _vector4))
  (bind _s_eventstruct_2 (Utilities|Struct|MakeS_EventStruct 0 1 "20.000000,10.000000,1.000000" _vector4_2))
  (bind (_moltypea _moltypeb _endlocation _endquat) (Utilities|Struct|BreakS_EventStruct _s_eventstruct))
  (bind (_moltypea_2 _moltypeb_2 _endlocation_2 _endquat_2) (Utilities|Struct|BreakS_EventStruct _s_eventstruct_2))
  (bind (_x _y _z _w) (Math|Vector4|BreakVector4 _endquat))
  (bind (_x_2 _y_2 _z_2) (Math|Vector|BreakVector _endlocation_2))
  (bind (_x_3 _y_3 _z_3 _w_2) (Math|Vector4|BreakVector4 _endquat_2))
  (bind (_x_4 _y_4 _z_4) (Math|Vector|BreakVector _endlocation))
  (bind (_canvas _size _context) (Rendering|BeginDrawCanvastoRenderTarget "/Game/NiagaraSystems/Niagara_MoleculeEmitter/RT_Events.RT_Events"))
  (for (_array_element _array_index) (Utilities|Array|MakeArray (Utilities|Struct|MakeLinearColor (Math|Conversions|ToFloat(Integer) _moltypea_2) (Math|Conversions|ToFloat(Integer) _moltypeb_2) 0.0 0.0) (Utilities|Struct|MakeLinearColor _x_2 _y_2 _z_2 0.0) (Utilities|Struct|MakeLinearColor _x_3 _y_3 _z_3 _w_2) (Utilities|Struct|MakeLinearColor (Math|Conversions|ToFloat(Integer) _moltypea) (Math|Conversions|ToFloat(Integer) _moltypeb) 0.0 0.0) (Utilities|Struct|MakeLinearColor _x_4 _y_4 _z_4 0.0) (Utilities|Struct|MakeLinearColor _x _y _z _w))
    (Canvas|DrawTexture :self _canvas :ScreenPosition (Math|Vector2D|MakeVector2D (Math|Conversions|ToFloat(Integer) _array_index) 0.0) :ScreenSize "(X=1.000000,Y=1.000000)" :CoordinateSize "(X=1.000000,Y=1.000000)" :RenderColor _array_element :BlendMode "BLEND_Opaque" :PivotPoint "(X=0.500000,Y=0.500000)"))
  (Rendering|EndDrawCanvastoRenderTarget _context))

(fn TempCreateEventStruct
  (params (MolTypeA :type Integer) (MolTypeB :type Integer) (EndLocation :type Vector) (EndQuat :type Vector%204%20Structure)))

(fn EventStructtoLinearColorArray
  (params (NewParam :type Vector%204%20Structure)))

(fn EventStructtoLinearColor
  (params (EventStruct :type S%20Event%20Struct%20Structure))
  (return ""))